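; Droplet actor that disappears when the player character touches it, or when the puddle (Flaque) actor reports a droplet touch.
; BeginPlay caches the first CharacterBP and Flaque found in the level.
; Box overlap with the character sets GoutteTouch, hides the Cube and disables collision; end overlap clears the flag after a short delay.
; Tick polls the Flaque's own GoutteTouch flag and applies the same hide and collision disable.
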(event `self.ReceiveTick`
  (params (DeltaSeconds :type "Float (single-precision)"))
  (bind _asflaque (cast `/Game/EnemyBP/Flaque` (`self.Flaque`)))
  (if (`/Game/EnemyBP/Flaque.GoutteTouch?` _asflaque)
    (`SceneComponent.SetHiddenInGame` (`self.Cube`) true false)
    (`self.SetActorEnableCollision` false)))

(event `self.ReceiveBeginPlay`
  (`self.GetCharacterBP`)
  (`self.GetFlaqueBP`))

(event `self.Box.OnComponentBeginOverlap`
  (params (OverlappedComponent :type "PrimitiveComponent Object Reference") (OtherActor :type "Actor Object Reference") (OtherComp :type "PrimitiveComponent Object Reference") (OtherBodyIndex :type Integer) (bFromSweep :type Boolean) (SweepResult :type "HitResult Structure (by ref)"))
  (if (== OtherActor (`self.CharacterBP`))
    (set `self.GoutteTouch?` true)
    (`SceneComponent.SetHiddenInGame` (`self.Cube`) true false)
    (`self.SetActorEnableCollision` false)))

(event `self.Box.OnComponentEndOverlap`
  (params (OverlappedComponent :type "PrimitiveComponent Object Reference") (OtherActor :type "Actor Object Reference") (OtherComp :type "PrimitiveComponent Object Reference") (OtherBodyIndex :type Integer))
  (if (== OtherActor (`self.CharacterBP`))
    (`KismetSystemLibrary.Delay` 0.2)
    (set `self.GoutteTouch?` false)))

(fn `GetCharacterBP`
  (bind _outactors (`GameplayStatics.GetAllActorsOfClass` "/Game/Character/CharacterBP.CharacterBP_C"))
  (set `self.CharacterBP` (`|GetArrayItem` _outactors)))

(fn `GetFlaqueBP`
  (bind _outactors (`GameplayStatics.GetAllActorsOfClass` "/Game/EnemyBP/Flaque.Flaque_C"))
  (set `self.Flaque` (`|GetArrayItem` _outactors)))

(fn `UserConstructionScript`)