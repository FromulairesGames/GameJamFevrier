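; PicBP is an enemy-folder actor that flags when the player character touches its collision box.
; On BeginPlay it caches the first CharacterBP instance found in the level.
; Box overlap by that character sets PicTouch to true, and end overlap clears it after a short delay.
; The file only maintains this flag and applies no effect to the character itself.
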(event `self.ReceiveBeginPlay`
  (bind _outactors (`GameplayStatics.GetAllActorsOfClass` "/Game/Character/CharacterBP.CharacterBP_C"))
  (set `self.CharacterBP` (`|GetArrayItem` _outactors)))

(event `self.Box.OnComponentBeginOverlap`
  (params (OverlappedComponent :type "PrimitiveComponent Object Reference") (OtherActor :type "Actor Object Reference") (OtherComp :type "PrimitiveComponent Object Reference") (OtherBodyIndex :type Integer) (bFromSweep :type Boolean) (SweepResult :type "HitResult Structure (by ref)"))
  (if (== OtherActor (`self.CharacterBP`))
    (set `self.PicTouch?` true)))

(event `self.Box.OnComponentEndOverlap`
  (params (OverlappedComponent :type "PrimitiveComponent Object Reference") (OtherActor :type "Actor Object Reference") (OtherComp :type "PrimitiveComponent Object Reference") (OtherBodyIndex :type Integer))
  (if (== OtherActor (`self.CharacterBP`))
    (`KismetSystemLibrary.Delay` 0.2)
    (set `self.PicTouch?` false)))

(fn `UserConstructionScript`)