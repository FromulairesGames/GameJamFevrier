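; Separate sprite actor that displays the 2D Paper2D animations of the CharacterBP character.
; On BeginPlay it caches the first CharacterBP in the level, then each Tick snaps itself to that character's SphereLoc.
; It polls the character's state flags to pick idle, run or jump flipbooks, or to reveal the separate MaxiRun and Hurt visuals.
; The hurt check runs ReverseFlipbook every frame to flip facing; HideForMaxiRun is never called.
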(event `self.ReceiveBeginPlay`
  (`self.GetCharacterBP`))

(event `self.ReceiveTick`
  (params (DeltaSeconds :type "Float (single-precision)"))
  (`self.SetFlipbookOnSphere`)
  (`|ExecutionSequence`
    (:`then_0`
      (`self.SetIdle`))
    (:`then_1`
      (`self.SetMaxiRunFlipbook`))
    (:`then_2`
      (`self.SetHurtFlipbook`))
    (:`then_3`
      (`self.SetJumpFlipbook`))))

(fn `GetCharacterBP`
  (bind _outactors (`GameplayStatics.GetAllActorsOfClass` "/Game/Character/CharacterBP.CharacterBP_C"))
  (set `self.Character` (`|GetArrayItem` _outactors)))

(fn `HideForMaxiRun`
  (bind _ascharacter_bp (cast `/Game/Character/CharacterBP` (`self.Character`)))
  (if (`/Game/Character/CharacterBP.Speed?` _ascharacter_bp)
    (`SceneComponent.SetHiddenInGame` (`self.PaperFlipbook`) true false)
    (else
      (`SceneComponent.SetHiddenInGame` (`self.PaperFlipbook`) false false))))

(fn `ReverseFlipbook`
  (bind _ascharacter_bp (cast `/Game/Character/CharacterBP` (`self.Character`)))
  (if (`/Game/Character/CharacterBP.Reverse?` _ascharacter_bp)
    (`self.K2_SetActorRotation` (struct))
    (else
      (`self.K2_SetActorRotation` (struct :`Pitch` 30.0 :`Yaw` -180.0)))))

(fn `SetFlipbookOnSphere`
  (bind _ascharacter_bp (cast `/Game/Character/CharacterBP` (`self.Character`)))
  (`self.K2_SetActorLocation` (`/Game/Character/CharacterBP.SphereLoc` _ascharacter_bp)))

(fn `SetHurtFlipbook`
  (bind _ascharacter_bp (cast `/Game/Character/CharacterBP` (`self.Character`)))
  (if (`/Game/Character/CharacterBP.Damage?` _ascharacter_bp)
    (`SceneComponent.SetHiddenInGame` (`self.Hurt`) false false)
    (`SceneComponent.SetHiddenInGame` (`self.MaxiRun`) true false)
    (`SceneComponent.SetHiddenInGame` (`self.PaperFlipbook`) true false)
    (`self.ReverseFlipbook`)
    (else
      (`SceneComponent.SetHiddenInGame` (`self.Hurt`) true false)
      (`self.ReverseFlipbook`))))

(fn `SetIdle`
  (bind _ascharacter_bp (cast `/Game/Character/CharacterBP` (`self.Character`)))
  (if (`/Game/Character/CharacterBP.Zero?` _ascharacter_bp)
    (`PaperFlipbookComponent.SetFlipbook` (`self.PaperFlipbook`) "/Game/CharacterAssets/IdleSprite/Idle.Idle")
    (else
      (`PaperFlipbookComponent.SetFlipbook` (`self.PaperFlipbook`) "/Game/CharacterAssets/Run.Run"))))

(fn `SetJumpFlipbook`
  (bind _ascharacter_bp (cast `/Game/Character/CharacterBP` (`self.Character`)))
  (if (`/Game/Character/CharacterBP.PressedJumpFB?` _ascharacter_bp)
    (`PaperFlipbookComponent.SetFlipbook` (`self.PaperFlipbook`) "/Game/CharacterAssets/Elan.Elan")))

(fn `SetMaxiRunFlipbook`
  (bind _ascharacter_bp (cast `/Game/Character/CharacterBP` (`self.Character`)))
  (if (`/Game/Character/CharacterBP.Speed?` _ascharacter_bp)
    (`SceneComponent.SetHiddenInGame` (`self.MaxiRun`) false false)
    (`SceneComponent.SetHiddenInGame` (`self.PaperFlipbook`) true false)
    (else
      (`SceneComponent.SetHiddenInGame` (`self.MaxiRun`) true false)
      (`SceneComponent.SetHiddenInGame` (`self.PaperFlipbook`) false false))))

(fn `UserConstructionScript`)