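; CharacterBP is a sphere-based player Blueprint that jumps when Z is pressed while a TriggerJumpBP reports touch.
; Each tick it stores the sphere's world location and looks up the first TriggerJumpBP actor in the level.
; On Z, it casts that actor, checks its Touch flag and applies a strong, mostly upward impulse to the sphere.
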(event `self.ReceiveTick`
  (params (DeltaSeconds :type "Float (single-precision)"))
  (`self.GetLocSphere`)
  (`self.GetTriggerJump`))

(event `Key|Z`
  (params (Key :type "Key Structure"))
  (:`Pressed`
    (bind _astrigger_jump_bp (cast `/Game/TriggerJumpBP` (`self.TriggerJump`)))
    (if (`/Game/TriggerJumpBP.Touch?` _astrigger_jump_bp)
      (`PrimitiveComponent.AddImpulse` (`self.Sphere`) (2000.0 0.0 60000.0) "None" false))))

(fn `GetLocSphere`
  (set `self.SphereLoc` (`SceneComponent.K2_GetComponentLocation` (`self.Sphere`))))

(fn `GetTriggerJump`
  (bind _outactors (`GameplayStatics.GetAllActorsOfClass` "/Game/TriggerJumpBP.TriggerJumpBP_C"))
  (set `self.TriggerJump` (`|GetArrayItem` _outactors)))

(fn `UserConstructionScript`)